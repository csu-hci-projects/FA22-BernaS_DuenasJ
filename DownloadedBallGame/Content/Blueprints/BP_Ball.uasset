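; BP_Ball is the player's physics ball, handling braking, camera control and jump recharging.
; StopMove brakes by zeroing max angular velocity and raising linear damping, with release and BeginPlay applying normal values.
; Inputs rotate and zoom the spring arm camera, toggling a zero-length "hamster" view or fixed top-down view.
; Any hit restores a spent jump on PC_SpeedBall with a landing sound, which also permits wall jumps.
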(event `InputAxis|Turn_Left/Right`
  (params (AxisValue :type "Float (single-precision)"))
  ;[1 1 1] Turn Left/Right
  (`self.AddControllerYawInput` AxisValue))

(event `InputAction|StopMove`
  (params (Key :type "Key Structure"))
  (bind _ball (`self.Ball`))
  ;[1 1 1] Stop Movement
  (:`Pressed`
    (`PrimitiveComponent.SetPhysicsMaxAngularVelocityInDegrees` _ball 0.0 false "None")
    (`PrimitiveComponent.SetLinearDamping` _ball 10.0))
  (:`Released`
    (`PrimitiveComponent.SetPhysicsMaxAngularVelocityInDegrees` _ball (`self.MaxAngVel`) false "None" :!label _label)
    (`PrimitiveComponent.SetLinearDamping` _ball 1.0)))

(event `InputAxis|Turn_Up/Down`
  (params (AxisValue :type "Float (single-precision)"))
  ;[1 1 1] Turn Left/Right
  (`self.AddControllerPitchInput` AxisValue))

(event `self.ReceiveBeginPlay`
  ;[1 1 1] Stop Movement
  (goto _label))

(event `InputAxisKey|MouseX`
  (params (AxisValue :type "Float (single-precision)"))
  ;[1 1 1] Move Springarm with cameraview
  (`SceneComponent.K2_AddRelativeRotation` (`self.SpringArm`) (`KismetMathLibrary.MakeRotator` 0.0 0.0 AxisValue) false false))

(event `self.ReceiveHit`
  (params (MyComp :type "PrimitiveComponent Object Reference") (Other :type "Actor Object Reference") (OtherComp :type "PrimitiveComponent Object Reference") (bSelfMoved :type Boolean) (HitLocation :type "Vector Structure") (HitNormal :type "Vector Structure") (NormalImpulse :type "Vector Structure") (Hit :type "HitResult Structure (by ref)"))
  ;[1 1 1] Reset Jump If Hit actor (Enables Wall Jumps- Intentional?)
  (bind _aspc_speed_ball (cast `/Game/Blueprints/PC_SpeedBall` (`GameplayStatics.GetPlayerController` 0)))
  (if (< (`/Game/Blueprints/PC_SpeedBall.NumJumps` _aspc_speed_ball) 1)
    (set `/Game/Blueprints/PC_SpeedBall.NumJumps` 1 _aspc_speed_ball)
    (`GameplayStatics.PlaySound2D` "/Game/SuperGrid/TutorialLevel/SoundEffects/Cue_Landing.Cue_Landing" 0.2 0.7 0.0 null null)))

(event `InputAxis|Zoom`
  (params (AxisValue :type "Float (single-precision)"))
  (bind _springarm (`self.SpringArm`))
  (bind _returnvalue (+ (* AxisValue -25.0) (`SpringArmComponent.TargetArmLength` _springarm)))
  ;[1 1 1] Zooming Camera in and out
  (if (`KismetMathLibrary.InRange_IntInt` (`KismetMathLibrary.FTrunc` _returnvalue) 100 1000)
    (set `SpringArmComponent.TargetArmLength` _returnvalue _springarm)))

(event `InputAction|HamsterMode`
  (params (Key :type "Key Structure"))
  (bind _springarm (`self.SpringArm`))
  ;[1 1 1] Zooming Camera in and out
  ;;[1 1 1] H pressed: toggle Hamster mode
  (:`Pressed`
    (if (< (`SpringArmComponent.TargetArmLength` _springarm) 10.0)
      (set `SpringArmComponent.TargetArmLength` 400.0 _springarm)
      (else
        (set `SpringArmComponent.TargetArmLength` 0.0 _springarm)))))

(event `InputAction|TopDownMode`
  (params (Key :type "Key Structure"))
  ;[1 1 1] J Pressed: toggle top-down
  (:`Pressed`
    (`self.TopDownModeToggle`)))

(fn `GetBallRef`
  (returns (Ball :type "/Game/Blueprints/BP_Ball Object Reference"))
  (return self))

(fn `GetBallRef2`
  (returns (BPBall2 :type "/Game/Blueprints/BP_Ball Object Reference"))
  (return null))

(fn `TopDownModeToggle`
  (bind _springarm (`self.SpringArm`))
  ;[1 1 1] Toggle, change spring arm length to set amount and put camera above ball looking down
  (if (`self.TopDown?`)
    (set `SpringArmComponent.bUsePawnControlRotation` true _springarm)
    (set `SpringArmComponent.TargetArmLength` 400.0 _springarm)
    (set `self.TopDown?` false)
    (else
      (set `SpringArmComponent.bUsePawnControlRotation` false _springarm)
      (set `SpringArmComponent.TargetArmLength` 1000.0 _springarm)
      (`SceneComponent.K2_SetRelativeRotation` _springarm (struct :`Pitch` -90.0 :`Yaw` 180.0) false false)
      (set `self.TopDown?` true))))

(fn `UserConstructionScript`)