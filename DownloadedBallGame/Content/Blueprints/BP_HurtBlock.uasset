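; BP_HurtBlock is a moving hazard that damages the player through the PC_SpeedBall controller when a BP_Ball hits it.
; Each tick it sweeps BadGuy along plus or minus SpeedDirection, accumulating the signed offset in VectorVariable.
; When that offset's Z reaches AmountToMove's Z, it resets the offset and flips direction; X, Y and absolute distance are not compared.
; Debug prints report the active path and both vectors.
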(event `self.ReceiveHit`
  (params (MyComp :type "PrimitiveComponent Object Reference") (Other :type "Actor Object Reference") (OtherComp :type "PrimitiveComponent Object Reference") (bSelfMoved :type Boolean) (HitLocation :type "Vector Structure") (HitNormal :type "Vector Structure") (NormalImpulse :type "Vector Structure") (Hit :type "HitResult Structure (by ref)"))
  (cast `/Game/Blueprints/BP_Ball` Other)
  (bind _aspc_speed_ball (cast `/Game/Blueprints/PC_SpeedBall` (`GameplayStatics.GetPlayerController` 0)))
  (`/Game/Blueprints/PC_SpeedBall.TakeDamage` _aspc_speed_ball (`self.DamageGiven`)))

(event `self.ReceiveTick`
  (params (DeltaSeconds :type "Float (single-precision)"))
  (bind _badguy (`self.BadGuy`))
  (bind _speed_direction (`self.Speed&Direction`))
  (bind _returnvalue (`SceneComponent.K2_GetComponentLocation` _badguy))
  (bind _returnvalue_2 (* -1.0 (`self.Speed&Direction`)))
  (if (`self.Bool`)
    (`SceneComponent.K2_SetWorldLocation` _badguy (+ _returnvalue _speed_direction) true false)
    (`KismetSystemLibrary.PrintString` "Path 1")
    (set `self.VectorVariable` (+ _speed_direction (`self.VectorVariable`)))
    (else
      (`SceneComponent.K2_SetWorldLocation` _badguy (+ _returnvalue _returnvalue_2) true false)
      (`KismetSystemLibrary.PrintString` "path 2")
      (set `self.VectorVariable` (+ _returnvalue_2 (`self.VectorVariable`)))))
  (bind _true_ (`self.GreaterThan(Vector)` 0.0))
  (if _true_
    (set `self.VectorVariable` (0.0 0.0 0.0))
    (if (`self.Bool`)
      (set `self.Bool` false)
      (else
        (set `self.Bool` true)))))

(fn `GreaterThan(Vector)`
  (params (X :type "Float (double-precision)") (Y :type "Float (double-precision)") (Z :type "Float (double-precision)"))
  (returns (`True?` :type Boolean))
  (bind (_amounttomove_x _amounttomove_y _amounttomove_z) (`KismetMathLibrary.BreakVector` (`self.AmountToMove`)))
  (bind (_vectorvariable_x _vectorvariable_y _vectorvariable_z) (`KismetMathLibrary.BreakVector` (`self.VectorVariable`)))
  (`KismetSystemLibrary.PrintString` (`KismetStringLibrary.Conv_VectorToString` (`self.VectorVariable`)))
  (`KismetSystemLibrary.PrintString` (`KismetStringLibrary.Conv_VectorToString` (`self.AmountToMove`)))
  (return (>= _vectorvariable_z _amounttomove_z)))

(fn `UserConstructionScript`)