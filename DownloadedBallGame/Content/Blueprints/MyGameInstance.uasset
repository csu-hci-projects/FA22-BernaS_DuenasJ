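; Game instance Blueprint that manages background music and the game's difficulty setting.
; StartMusic stops any valid existing sound, then creates, stores and plays a 2D sound with auto-destroy off and optional persistence across level transitions.
; Raise and lower functions step GameDifficulty one level at a time within a clamped three-level range.
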(fn `LowerDifficulty`
  (bind _gamedifficulty (`self.GameDifficulty`))
  ;[1 1 1] If not lowest Difficulty, lower it
  (if (> _gamedifficulty 0)
    (set `self.GameDifficulty` (- _gamedifficulty 1))))

(fn `RaiseDifficulty`
  (bind _gamedifficulty (`self.GameDifficulty`))
  ;[1 1 1] If not highest Difficulty, raise it
  (if (< _gamedifficulty 2)
    (set `self.GameDifficulty` (+ _gamedifficulty 1))))

(fn `StartMusic`
  (params (Sound :type "SoundBase Object Reference") (VolumeMultiplier :type "Float (single-precision)") (bPersistAcrossLevelTransition :type Boolean))
  ;[1 1 1] When called at start of game, if sound is already playing then stop it and start again, otherwise just play the sound
  (`/Engine/EditorBlueprintResources/StandardMacros.IsValid` (stale _output_get)
    (:`Is Valid`
      (`AudioComponent.Stop` (stale _output_get)))
    (:`Is Not Valid`
      _))
  (bind _returnvalue (`GameplayStatics.CreateSound2D` Sound VolumeMultiplier 1.0 0.0 null bPersistAcrossLevelTransition false))
  (bind _output_get (set `self.Sound` _returnvalue))
  (`AudioComponent.Play` _output_get 0.0))