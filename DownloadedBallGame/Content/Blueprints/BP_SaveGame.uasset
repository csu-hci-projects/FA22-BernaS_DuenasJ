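; BP_SaveGame holds the ball game's high score, lives, score and current level, and contains logic that resets a run when StartGame is pressed.
; An existing slot save is loaded and reset to starting values while keeping its high score; otherwise a new save is created with zero high score.
; Both branches write back to the same slot.
; A player controller cast is unconnected, and LoadGameMacro has no logic.
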(event `InputAction|StartGame`
  (params (Key :type "Key Structure"))
  (:`Pressed`
    (bind _returnvalue (`GameplayStatics.DoesSaveGameExist` "Slot1"))
    (if _returnvalue
      (bind _returnvalue_2 (`GameplayStatics.LoadGameFromSlot` "Slot1"))
      (bind _asbp_save_game (cast `/Game/Blueprints/BP_SaveGame` _returnvalue_2))
      (set `/Game/Blueprints/BP_SaveGame.HighScore` (`/Game/Blueprints/BP_SaveGame.HighScore` _asbp_save_game) _asbp_save_game)
      (set `/Game/Blueprints/BP_SaveGame.CurrLives` 3 _asbp_save_game)
      (set `/Game/Blueprints/BP_SaveGame.CurrScore` 0 _asbp_save_game)
      (set `/Game/Blueprints/BP_SaveGame.CurrLevel` "Level_BallGame_1" _asbp_save_game)
      (`GameplayStatics.SaveGameToSlot` _asbp_save_game "Slot1")
      (else
        (bind _returnvalue_3 (`GameplayStatics.CreateSaveGameObject` "BP_SaveGame_C"))
        (set `/Game/Blueprints/BP_SaveGame.HighScore` 0 _returnvalue_3)
        (set `/Game/Blueprints/BP_SaveGame.CurrLives` 3 _returnvalue_3)
        (set `/Game/Blueprints/BP_SaveGame.CurrScore` 0 _returnvalue_3)
        (set `/Game/Blueprints/BP_SaveGame.CurrLevel` "Level_BallGame_1" _returnvalue_3)
        (`GameplayStatics.SaveGameToSlot` _returnvalue_3 "Slot1")))))