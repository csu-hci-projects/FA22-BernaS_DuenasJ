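; BP_Star is a collectible star pickup that spins in place until the ball touches it.
; On overlap with a BP_Ball, it calls CollectedStar on the PC_SpeedBall player controller, then destroys itself.
; Each tick, SpinFunction adds a fixed yaw step to the static mesh's relative rotation, so spin speed depends on frame rate.
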(event `self.ReceiveActorBeginOverlap`
  (params (OtherActor :type "Actor Object Reference"))
  ;[1 1 1] If ball overlaps, call collected star function
  (cast `/Game/Blueprints/BP_Ball` OtherActor)
  (bind _aspc_speed_ball (cast `/Game/Blueprints/PC_SpeedBall` (`GameplayStatics.GetPlayerController` 0)))
  (`/Game/Blueprints/PC_SpeedBall.CollectedStar` _aspc_speed_ball)
  (`self.K2_DestroyActor`))

(event `self.ReceiveTick`
  (params (DeltaSeconds :type "Float (single-precision)"))
  ;[1 1 1] Spin
  (`self.SpinFunction` 0.5))

(fn `SpinFunction`
  (params (SpinAmount :type "Float (double-precision)"))
  (bind _staticmesh (`self.StaticMesh`))
  (bind (_relativerotation_roll _relativerotation_pitch _relativerotation_yaw) (`KismetMathLibrary.BreakRotator` (`SceneComponent.RelativeRotation` _staticmesh)))
  ;[1 1 1] Add rotation, to make it spin
  (`SceneComponent.K2_SetRelativeRotation` _staticmesh (`KismetMathLibrary.MakeRotator` 0.0 0.0 (+ SpinAmount _relativerotation_yaw)) false false))

(fn `UserConstructionScript`)