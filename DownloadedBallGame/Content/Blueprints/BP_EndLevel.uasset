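; BP_EndLevel is a level-end trigger that adds to the saved high score when a BP_Ball overlaps it.
; On overlap it loads the BP_SaveGame in Slot1 and raises HighScore by a fixed amount, or creates a save starting at that amount.
; Both branches save back to Slot1, passing HighScore as the UserIndex, whereas the existence check and load use user index 0.
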(event `self.ReceiveActorBeginOverlap`
  (params (OtherActor :type "Actor Object Reference"))
  (cast `/Game/Blueprints/BP_Ball` OtherActor)
  (bind _returnvalue (`GameplayStatics.DoesSaveGameExist` "Slot1"))
  (if _returnvalue
    (bind _returnvalue_2 (`GameplayStatics.LoadGameFromSlot` "Slot1"))
    (bind _asbp_save_game (cast `/Game/Blueprints/BP_SaveGame` _returnvalue_2))
    (bind _output_get (set `/Game/Blueprints/BP_SaveGame.HighScore` (+ (`/Game/Blueprints/BP_SaveGame.HighScore` _asbp_save_game) 10) _asbp_save_game))
    (`GameplayStatics.SaveGameToSlot` _asbp_save_game "Slot1" _output_get)
    (else
      (bind _returnvalue_3 (`GameplayStatics.CreateSaveGameObject` "/Game/Blueprints/BP_SaveGame.BP_SaveGame_C"))
      (bind _output_get_2 (set `/Game/Blueprints/BP_SaveGame.HighScore` 10 _returnvalue_3))
      (`GameplayStatics.SaveGameToSlot` _returnvalue_3 "Slot1" _output_get_2))))

(fn `UserConstructionScript`)